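; BP_VortexWeapon is a projectile-style weapon actor that becomes a stationary vortex, pulling in and damaging enemies.
; After a short delay on BeginPlay, it enables its query-only sphere, stops projectile movement and starts a looping timer.
; Each tick damages overlapping BP_Base_Enemy actors and launches them toward the center with distance-scaled velocity.
; The parent BeginPlay is never called, and the Hit event is left empty.
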(event Custom|VortexTick
  (for _array_element (Collision|GetOverlappingActors (Variables|Default|GetSphere) "/Game/SurvivorsTemplate/Blueprints/Enemies/BP_Base_Enemy.BP_Base_Enemy_C" :!class /Script/Engine.PrimitiveComponent)
    (Game|Damage|ApplyDamage _array_element 1.0 0 0)
    (bind _ascharacter (Utilities|Casting|CastToCharacter _array_element))
    (Character|LaunchCharacter _ascharacter (* (- (Transformation|GetActorLocation) (Transformation|GetActorLocation _array_element)) 5.0) true true)))

(event Collision|EventActorBeginOverlap
  (params (OtherActor :type Actor%20Object%20Reference))
  (|CallParentFunction OtherActor) ; This node is disabled and will not be called.\nDrag off pins to build functionality.
)

(event EventTick
  (params (DeltaSeconds :type Float%20%28single-precision%29))
  (|CallParentFunction DeltaSeconds) ; This node is disabled and will not be called.\nDrag off pins to build functionality.
)

(event EventBeginPlay
  (Collision|SetCollisionEnabled (Variables|Default|GetSphere) "NoCollision")
  (Utilities|FlowControl|Delay 0.3)
  (Collision|SetCollisionEnabled (Variables|Default|GetSphere) "QueryOnly")
  (Components|Movement|StopMovementImmediately (Variables|Default|GetProjectileMovement))
  (Utilities|Time|SetTimerbyEvent (delegate Custom|VortexTick) 0.3 true))

(event Collision|EventHit
  (params (MyComp :type Primitive%20Component%20Object%20Reference) (Other :type Actor%20Object%20Reference) (OtherComp :type Primitive%20Component%20Object%20Reference) (bSelfMoved :type Boolean) (HitLocation :type Vector :default "0, 0, 0") (HitNormal :type Vector :default "0, 0, 0") (NormalImpulse :type Vector :default "0, 0, 0") (Hit :type Hit%20Result%20Structure%20%28by%20ref%29)))

(fn ConstructionScript
  (|CallParentFunction))